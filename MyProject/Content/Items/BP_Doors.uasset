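; Door actor that swings open or closed when BP_Character enters its Open trigger.
; ToOpen plays or reverses a timeline based on IsClose, driving the Cube's world yaw up to OpenAngle.
; When the timeline finishes, it flips IsClose and clears Locker after a short delay.
; Locker is meant to block repeat triggers by printing a wait message, but this graph never sets it true.
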(event `self.Open.OnComponentBeginOverlap`
  (params (OverlappedComponent :type "PrimitiveComponent Object Reference") (OtherActor :type "Actor Object Reference") (OtherComp :type "PrimitiveComponent Object Reference") (OtherBodyIndex :type Integer) (bFromSweep :type Boolean) (SweepResult :type "HitResult Structure (by ref)"))
  ;[1 1 1] reconnaitre le joueur et vérifier si le timer est terminé pour pas lancer l'ouverture plusieurs fois d'affiler
  (cast `/Game/ThirdPerson/Blueprints/BP_Character` OtherActor)
  (if (`self.Locker`)
    (`KismetSystemLibrary.PrintString` "Wait")
    (else
      (`self.ToOpen`))))

(event `ToOpen`
  (bind _cube (`self.Cube`))
  (bind (_returnvalue_roll _returnvalue_pitch) (`KismetMathLibrary.BreakRotator` (`SceneComponent.K2_GetComponentRotation` _cube)))
  ;[0.1539 0.9403 1] Event d'ouverture
  ;;[1 0.7494 0.4222] On vérifie si la porte est déjà ouvert pour déterminer le sens d'ouverture
  (if (`self.IsClose`)
    (bind (_direction _newtrack_0) (`Timeline|Timeline` :!via `PlayFromStart` :!label _label)
      (:`Update`
        (`SceneComponent.K2_SetWorldRotation` _cube (`KismetMathLibrary.MakeRotator` _returnvalue_roll _returnvalue_pitch (* _newtrack_0 (`self.OpenAngle`))) false false))
      (:`Finished`
        ;;[0.1238 1 0] Gérer le timer et le sens de d'ouverture de la porte
        (if (`self.IsClose`)
          (set `self.IsClose` false)
          (`KismetSystemLibrary.Delay` 3.0)
          (set `self.Locker` false)
          (else
            (set `self.IsClose` true)
            (`KismetSystemLibrary.Delay` 3.0)
            (set `self.Locker` false)))))
    (else
      (goto _label :!via `Reverse`))))

(fn `UserConstructionScript`)